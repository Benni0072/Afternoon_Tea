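; BP_Interact_Dialogue is an interactable Blueprint that toggles a dialogue UI each time its Interact event fires.
; The first opening creates a WB_Dialogue widget, adds it to the viewport and plays its Letteranimation.
; Later toggles reuse that cached widget and only switch its visibility, so the animation is not replayed.
; Nodes for clearing the widget reference and reversing the animation are present but never run.
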(event EventInteract
  (bind _output_get (Variables|Default|SetIs%20UI%20Open (not (Variables|Default|GetIs%20UI%20Open))))
  (if _output_get
    (Utilities|IsValid (Variables|Default|GetUI)
      (:Is%20Valid
        _)
      (:Is%20Not%20Valid
        (bind _returnvalue (UserInterface|CreateWidget "/Game/UI/WB_Dialogue.WB_Dialogue_C"))
        (bind _output_get_2 (Variables|Default|SetUI _returnvalue))
        (UserInterface|Viewport|AddtoViewport _output_get_2 0)
        (UserInterface|Animation|PlayAnimation (Variables|Default|GetUI) (Variables|/Game/UI/WB_Dialogue.WB_Dialogue_C|GetLetteranimation _output_get_2) 0.0 1 "Forward" 1.0 false)))
    (Widget|SetVisibility _output_get_2 "Visible")
    (else
      (Utilities|IsValid (Variables|Default|GetUI)
        (:Is%20Valid
          (Widget|SetVisibility _output_get_2 "Hidden"))))))

(fn ConstructionScript
  (|CallParentFunction))