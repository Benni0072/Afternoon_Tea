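; Player controller that adds the third-person Enhanced Input mapping context and caches the possessed BP_ThirdPersonCharacter.
; It forwards move, camera, dash, interact and pause input to that character, with the teleport action calling Respawn.
; Jump uses a DoOnce reset on release to fire once per press, saving the last velocity and toggling the character's gravity scale between press and release.
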(event Input|EnhancedActionEvents|EnhancedInputActionIA_Move
  (params (ActionValue :type Vector%202D%20Structure) (ElapsedSeconds :type Float%20%28double-precision%29) (TriggeredSeconds :type Float%20%28double-precision%29) (InputAction :type Input%20Action%20Object%20Reference :default "/Game/Input/InputActions/IA_Move.IA_Move"))
  (Default|MoveinWorldDirection (Variables|Default|GetPossessedThirdPersonCharacter) (Math|Vector|MakeVector (.x ActionValue) (.y ActionValue) 0.0)))

(event Input|EnhancedActionEvents|EnhancedInputActionIA_RotateCamera
  (params (ActionValue :type Vector%202D%20Structure) (ElapsedSeconds :type Float%20%28double-precision%29) (TriggeredSeconds :type Float%20%28double-precision%29) (InputAction :type Input%20Action%20Object%20Reference :default "/Game/Input/InputActions/IA_RotateCamera.IA_RotateCamera"))
  (bind _possessedthirdpersoncharacter (Variables|Default|GetPossessedThirdPersonCharacter))
  (Pawn|Input|AddControllerYawInput _possessedthirdpersoncharacter (.x ActionValue))
  (Pawn|Input|AddControllerPitchInput _possessedthirdpersoncharacter (.y ActionValue)))

(event Input|EnhancedActionEvents|EnhancedInputActionIA_Jump
  (params (ActionValue :type Boolean) (ElapsedSeconds :type Float%20%28double-precision%29) (TriggeredSeconds :type Float%20%28double-precision%29) (InputAction :type Input%20Action%20Object%20Reference :default "/Game/Input/InputActions/IA_Jump.IA_Jump"))
  (bind _possessedthirdpersoncharacter (Variables|Default|GetPossessedThirdPersonCharacter))
  (:Triggered
    (if (Character|CanJump _possessedthirdpersoncharacter)
      (Utilities|FlowControl|DoOnce false :!label _label
        (:Completed
          (Character|Jump _possessedthirdpersoncharacter)
          (Default|SaveLastVel _possessedthirdpersoncharacter)
          (Default|SetGravityScale _possessedthirdpersoncharacter true)))))
  (:Completed
    (Default|SetGravityScale (Variables|Default|GetPossessedThirdPersonCharacter) false)
    (goto _label Reset)))

(event Input|EnhancedActionEvents|EnhancedInputActionIA_Dash
  (params (ActionValue :type Boolean) (ElapsedSeconds :type Float%20%28double-precision%29) (TriggeredSeconds :type Float%20%28double-precision%29) (InputAction :type Input%20Action%20Object%20Reference :default "/Game/Input/InputActions/IA_Dash.IA_Dash"))
  (Default|Dash (Variables|Default|GetPossessedThirdPersonCharacter)))

(event Input|EnhancedActionEvents|EnhancedInputActionIA_Teleport
  (params (ActionValue :type Boolean) (ElapsedSeconds :type Float%20%28double-precision%29) (TriggeredSeconds :type Float%20%28double-precision%29) (InputAction :type Input%20Action%20Object%20Reference :default "/Game/Input/InputActions/IA_Teleport.IA_Teleport"))
  (Default|Respawn (Variables|Default|GetPossessedThirdPersonCharacter)))

(event Input|EnhancedActionEvents|EnhancedInputActionIA_Interact
  (params (ActionValue :type Boolean) (ElapsedSeconds :type Float%20%28double-precision%29) (TriggeredSeconds :type Float%20%28double-precision%29) (InputAction :type Input%20Action%20Object%20Reference :default "/Game/Input/InputActions/IA_Interact.IA_Interact"))
  (Default|TryInteract (Variables|Default|GetPossessedThirdPersonCharacter)))

(event Input|EnhancedActionEvents|EnhancedInputActionIA_Pause
  (params (ActionValue :type Boolean) (ElapsedSeconds :type Float%20%28double-precision%29) (TriggeredSeconds :type Float%20%28double-precision%29) (InputAction :type Input%20Action%20Object%20Reference :default "/Game/Input/InputActions/IA_Pause.IA_Pause"))
  (Default|PauseMenu (Variables|Default|GetPossessedThirdPersonCharacter)))

(event EventPossess
  (params (PossessedPawn :type Pawn%20Object%20Reference))
  (bind _asbp_third_person_character (Utilities|Casting|CastToBP_ThirdPersonCharacter PossessedPawn))
  (Variables|Default|SetPossessedThirdPersonCharacter _asbp_third_person_character))

(event EventBeginPlay
  (Input|AddMappingContext (PlayerController|LocalPlayerSubsystems|GetEnhancedInputLocalPlayerSubsystem) "/Game/Input/IMC_ThirdPersonCharacter.IMC_ThirdPersonCharacter" 0 "(bIgnoreAllPressedKeysUntilRelease=True,bForceImmediately=False,bNotifyUserSettings=False)"))

(fn ConstructionScript)