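; BP_InteractMusic is an interactable music player that cycles through three songs and an empty slot.
; BeginPlay and each Interact call PlayNextSong, which advances a wrapping index, sets the selected sound on its Audio component and calls Play.
; Actor overlap toggles custom depth rendering on its Cube, with no filter on the overlapping actor.
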(event EventBeginPlay
  (CallFunction|PlayNextSong))

(event Collision|EventActorBeginOverlap
  (params (OtherActor :type Actor%20Object%20Reference))
  (if true
    (Rendering|SetRenderCustomDepth (Variables|Default|GetCube) true)))

(event Collision|EventActorEndOverlap
  (params (OtherActor :type Actor%20Object%20Reference))
  (if true
    (Rendering|SetRenderCustomDepth (Variables|Default|GetCube) false)))

(event EventInteract
  (CallFunction|PlayNextSong))

(fn ConstructionScript
  (|CallParentFunction))

(fn PlayNextSong
  (CallFunction|IncrementMusicIndex)
  (Audio|Components|Audio|SetSound (Variables|Default|GetAudio) (Utilities|Select :Index (Variables|Default|GetMusicIndex) :Option%200 "/Game/Sound/Music/ES_Once_Upon_a_Road_-_Bladverk_Band.ES_Once_Upon_a_Road_-_Bladverk_Band" :Option%201 "/Game/Sound/Music/ES_The_Calling_Card_-_Martin_Landstrom.ES_The_Calling_Card_-_Martin_Landstrom" :Option%202 "/Game/Sound/Music/ES_Hollow_Stone_-_Daniel_Fridell.ES_Hollow_Stone_-_Daniel_Fridell" :Option%203 0))
  (Audio|Components|Audio|Play (Variables|Default|GetAudio) 0.0))

(fn IncrementMusicIndex
  (bind _output_get (Variables|Default|SetMusicIndex (+ (Variables|Default|GetMusicIndex) 1)))
  (if (> _output_get 3)
    (Variables|Default|SetMusicIndex 0)))