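; Collectible cookie pickup, a child Blueprint that extends a parent collectible with its own collect animation and collection response.
; On collection it calls OnCollectedCooky on the ThirdPersonCharacter's BPWWidget.
; The collect animation event plays a timeline that yaws the Pivot, scaled by AnimationSpeed, then destroys the actor when finished.
; Tick and the construction script only forward to the parent.
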(event Custom|EventPlayCollectAnimation
  (bind _newtrack_0 (Timeline|Timeline_0 Play)
    (:Update
      (Transformation|SetRelativeRotation (Variables|Default|GetPivot) (Math|Rotator|MakeRotator 0.0 0.0 (* _newtrack_0 (Variables|Default|GetAnimationSpeed))) false false))
    (:Finished
      (Actor|DestroyActor))))

(event EventOnCollected
  (params (ThirdPersonCharacter :type BP%20Third%20Person%20Character%20Object%20Reference))
  (Default|OnCollectedCooky (Variables|/Game/BP/BP_ThirdPersonCharacter.BP_ThirdPersonCharacter_C|GetBPW_Widget ThirdPersonCharacter)))

(event EventTick
  (params (DeltaSeconds :type Float%20%28single-precision%29))
  (|CallParentFunction DeltaSeconds))

(fn ConstructionScript
  (|CallParentFunction))