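; BP_Respawnpoint is a checkpoint actor that sets where the player character respawns.
; On overlap, it registers itself as the Spawnpoint on the player's BP_ThirdPersonCharacter and reveals its Niagara effect.
; A DoOnce plays a twinkle sound only on the first activation.
; GetRespawnLocRot returns the RespawnPivot component's world location and rotation as the respawn transform.
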(event Collision|EventActorBeginOverlap
  (params (OtherActor :type Actor%20Object%20Reference))
  (bind _asbp_third_person_character (Utilities|Casting|CastToBP_ThirdPersonCharacter (Game|Player|GetPlayerPawn 0)))
  (Variables|/Game/BP/BP_ThirdPersonCharacter.BP_ThirdPersonCharacter_C|SetSpawnpoint _asbp_third_person_character self)
  (Development|SetHiddeninGame (Variables|Default|GetNiagara) false false)
  (Utilities|FlowControl|DoOnce false
    (:Completed
      (Audio|PlaySound2D "/Game/Sound/SFX/Checkpoint/charming-twinkle-sound-for-fantasy-and-magic-250240.charming-twinkle-sound-for-fantasy-and-magic-250240" 1.0 1.0 0.0 0 0))))

(fn ConstructionScript)

(fn GetRespawnLocRot
  (bind _respawnpivot (Variables|Default|GetRespawnPivot))
  (return (Transformation|GetWorldLocation _respawnpivot) (Transformation|GetWorldRotation _respawnpivot)))