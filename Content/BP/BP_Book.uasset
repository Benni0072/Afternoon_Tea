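; BP_Book is an actor that rolls its static mesh, likely toppling a book, when a dashing player character hits it.
; Its Hit event casts to BP_ThirdPersonCharacter, checks IsDashing and passes through a DoOnce, so the reaction fires only once.
; A timeline track scaled by the Radius variable drives the mesh's relative roll.
; Unconnected nodes for actor rotation, a level sequence and destruction never run.
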(event Collision|EventHit
  (params (MyComp :type Primitive%20Component%20Object%20Reference) (Other :type Actor%20Object%20Reference) (OtherComp :type Primitive%20Component%20Object%20Reference) (bSelfMoved :type Boolean) (HitLocation :type Vector :default "0, 0, 0") (HitNormal :type Vector :default "0, 0, 0") (NormalImpulse :type Vector :default "0, 0, 0") (Hit :type Hit%20Result%20Structure%20%28by%20ref%29))
  (bind _asbp_third_person_character (Utilities|Casting|CastToBP_ThirdPersonCharacter Other))
  (if (Variables|/Game/BP/BP_ThirdPersonCharacter.BP_ThirdPersonCharacter_C|GetIsDashing _asbp_third_person_character)
    (Utilities|FlowControl|DoOnce false
      (:Completed
        (bind _newtrack_0 (Timeline|Timeline Play)
          (:Update
            (Transformation|SetRelativeRotation (Variables|Default|GetStaticMesh) (Math|Rotator|MakeRotator (* _newtrack_0 (Variables|Default|GetRadius)) 0.0 0.0) false false)))))))

(fn ConstructionScript)