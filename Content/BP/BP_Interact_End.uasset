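; BP_Interact_End is an interactable cup that ends the level and opens the credits.
; Actor overlap toggles custom depth rendering on the Cup component while something is in range.
; The Interact event switches the first player to UI-only input, fades the camera out and holds it, then loads the credits level once the fade delay finishes.
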(event Collision|EventActorEndOverlap
  (params (OtherActor :type Actor%20Object%20Reference))
  (if true
    (Rendering|SetRenderCustomDepth (Variables|Default|Get%20%20%20%20Cup) false)))

(event Collision|EventActorBeginOverlap
  (params (OtherActor :type Actor%20Object%20Reference))
  (if true
    (Rendering|SetRenderCustomDepth (Variables|Default|Get%20%20%20%20Cup) true)))

(event EventInteract
  (Input|SetInputModeUIOnly (Game|GetPlayerController 0) 0 "DoNotLock" true)
  (CameraFades|StartCameraFade :self (Game|GetPlayerCameraManager 0) :ToAlpha 1.0 :Duration 1.5 :bHoldWhenFinished true)
  (Utilities|FlowControl|Delay 1.5)
  (Game|OpenLevel(byObjectReference) "/Game/Maps/CreditsLvl.CreditsLvl"))

(fn ConstructionScript
  (|CallParentFunction))